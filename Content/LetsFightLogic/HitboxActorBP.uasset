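; HitboxActorBP is a hitbox actor for a fighting game that displays a strike or hurtbox volume and damages characters it overlaps.
; SpawnHitBox sets the indicator's material by hitbox type, moves it to the hitbox location, makes it visible and runs CheckCollision.
; CheckCollision makes a single overlap query for LetsFightCharacter actors, skips the owner and passes the hitbox damage to each one's DetermineHealth, regardless of type.
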(event Custom|SpawnHitBox
  (switch Utilities|FlowControl|Switch|SwitchonHurtBox_Type (Variables|Default|GethitBoxType)
    (:NewEnumerator0
      (Rendering|Material|SetMaterial (Variables|Default|GetHitboxIndicator) 0 "/Game/LetsFightLogic/Materials/M_StrikeHitBox.M_StrikeHitBox"))
    (:NewEnumerator1
      (Rendering|Material|SetMaterial (Variables|Default|GetHitboxIndicator) 0 "/Game/LetsFightLogic/Materials/M_Hurtbox.M_Hurtbox")))
  (Transformation|SetWorldLocation (Variables|Default|GetHitboxIndicator) (Variables|Default|GethitBoxLocation) false false)
  (Rendering|SetVisibility (Variables|Default|GetHitboxIndicator) true false)
  (CallFunction|CheckCollision))

(event Custom|CheckCollision
  (for _array_element (Collision|GetOverlappingActors "/Game/ThirdPersonBP/Blueprints/LetsFightCharacter.LetsFightCharacter_C" :!class /Script/Engine.Actor)
    (if (!= _array_element (Components|GetOwner))
      (bind _aslets_fight_character (Utilities|Casting|CastToLetsFightCharacter _array_element))
      (Default|DetermineHealth _aslets_fight_character (Variables|Default|GethitBoxDamage)))))

(event EventBeginPlay)

(event Collision|EventActorBeginOverlap
  (params (OtherActor :type Actor%20Object%20Reference)))

(event EventTick
  (params (DeltaSeconds :type Float%20%28single-precision%29)))

(fn ConstructionScript)